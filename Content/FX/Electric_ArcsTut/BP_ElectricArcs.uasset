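; Electric arc effect actor that draws a beam toward an End point, with two spark emitters oriented along the Start-to-End line.
; Tick feeds End's world location into the beam's BeamEnd parameter and opposite Start/End difference vectors into the sparks' Orientation.
; The construction script also sets these, but orients sparks from Start's location against a zero vector instead of End.
; A Movement timeline that would offset both points never runs.
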(event EventTick
  (params (DeltaSeconds :type Float%20%28single-precision%29))
  (bind _end (Variables|Default|GetEnd))
  (bind _start (Variables|Default|GetStart))
  (bind _returnvalue (Transformation|GetWorldLocation _start))
  (bind _returnvalue_2 (Transformation|GetWorldLocation _end))
  (bind _returnvalue_3 (- _returnvalue _returnvalue_2))
  (Effects|Components|ParticleSystem|SetVectorParameter (Variables|Default|GetElectricArcs) "BeamEnd" _returnvalue_2)
  (Effects|Components|ParticleSystem|SetVectorParameter (Variables|Default|GetSparks_01) "Orientation" (* _returnvalue_3 -1.0))
  (Effects|Components|ParticleSystem|SetVectorParameter (Variables|Default|GetSparks_02) "Orientation" _returnvalue_3))

(fn ConstructionScript
  (bind _start (Variables|Default|GetStart))
  (bind _returnvalue (Transformation|GetWorldLocation _start))
  (bind _returnvalue_2 (- _returnvalue ""))
  (Effects|Components|ParticleSystem|SetVectorParameter (Variables|Default|GetElectricArcs) "BeamEnd" (Transformation|GetWorldLocation (Variables|Default|GetEnd)))
  (Effects|Components|ParticleSystem|SetVectorParameter (Variables|Default|GetSparks_01) "Orientation" (* _returnvalue_2 -1.0))
  (Effects|Components|ParticleSystem|SetVectorParameter (Variables|Default|GetSparks_02) "Orientation" _returnvalue_2))