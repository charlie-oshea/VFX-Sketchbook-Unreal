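; BP_Aurora is an aurora borealis effect actor that lays a mesh with the aurora material along an editable spline.
; The construction script measures the mesh's X length from its bounding box and divides the spline length by it to set the segment count.
; Each segment becomes an X-forward spline mesh component, with endpoints sampled by distance and tangents clamped to the mesh length for continuous bending.
; The event graph has no active logic.
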(event EventBeginPlay)

(event Collision|EventActorBeginOverlap
  (params (OtherActor :type Actor%20Object%20Reference)))

(event EventTick
  (params (DeltaSeconds :type Float%20%28single-precision%29)))

(fn ConstructionScript
  (bind _mesh (Variables|Default|GetMesh))
  (bind _returnvalue (StaticMesh|GetBoundingBox _mesh))
  ;[1 0.05805 0.9559] Get X length of mesh
  (Variables|Default|SetX_Length (.x (+ (Math|Vector|VectorGetAbs (.min _returnvalue)) (Math|Vector|VectorGetAbs (.max _returnvalue)))))
  ;[1 0.03103 0.05092] Loop over points in spline
  (for _index (range 0 (Math|Float|Truncate (/ (Spline|GetSplineLength (Variables|Default|GetSpline)) (Variables|Default|GetX_Length))))
    ;[0.08683 1 0.1237] Set up mesh for spline section
    (bind _returnvalue_2 (AddComponent|AddSplineMeshComponent false))
    (SplineMesh|SetForwardAxis _returnvalue_2 "X" true)
    (Components|StaticMesh|SetStaticMesh _returnvalue_2 (Variables|Default|GetMesh))
    (Rendering|Material|SetMaterial _returnvalue_2 0 (Variables|Default|GetAuroraMaterial))
    (SplineMesh|SetStartandEnd _returnvalue_2 (Spline|GetLocationatDistanceAlongSpline (Variables|Default|GetSpline) (* _index (Variables|Default|GetX_Length)) "Local") (Math|Vector|ClampVectorSize (Spline|GetTangentatDistanceAlongSpline (Variables|Default|GetSpline) (* _index (Variables|Default|GetX_Length)) "Local") 0.0 (Variables|Default|GetX_Length)) (Spline|GetLocationatDistanceAlongSpline (Variables|Default|GetSpline) (* (+ _index 1) (Variables|Default|GetX_Length)) "Local") (Math|Vector|ClampVectorSize (Spline|GetTangentatDistanceAlongSpline (Variables|Default|GetSpline) (* (+ _index 1) (Variables|Default|GetX_Length)) "Local") 0.0 (Variables|Default|GetX_Length)) true :!class /Script/Engine.SplineMeshComponent)))